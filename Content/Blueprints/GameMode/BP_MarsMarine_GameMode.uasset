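; Game mode for Mars Marine that runs waves of BP_Alien enemies.
; SetupNewWave starts a looping timer that spawns aliens at random TargetPoints until AlienSpawnsRemaining reaches zero.
; RegisterAlienDeath removes tracked aliens and, once none remain alive or pending, triggers the next wave after a delay.
; StartNewWave adds multiplier-based difficulty scaling but is not called here; SetupNewWave never resets the spawn count.
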(event `self.ReceiveBeginPlay`
  (`KismetSystemLibrary.Delay` 2.0)
  (`self.Setup New Wave`))

(event `Spawn Wave`
  (`self.Spawn Alien`))

(event `End Wave`
  (`KismetSystemLibrary.Delay` 2.0)
  (`self.Setup New Wave`))

(fn `Getrandomspawnpoint`
  (returns (`Spawn Point` :type "TargetPoint Object Reference"))
  (bind _outactors (`GameplayStatics.GetAllActorsOfClass` "/Script/Engine.TargetPoint"))
  (return (`|GetArrayItem` _outactors (`KismetMathLibrary.RandomIntegerInRange` 0 (`KismetArrayLibrary.Array_LastIndex` _outactors)))))

(fn `increasewavediff`
  (bind _output_get (set `self.Wave Difficulty` (`KismetMathLibrary.Round` (* (`self.Wave Difficulty`) (`self.DifMulti`)))))
  (set `self.Alien Spawns Remaining` _output_get))

(fn `isWaveComplete`
  (returns (ReturnValue :type Boolean))
  (return (and (== (`KismetArrayLibrary.Array_Length` (`self.Aliens`)) 0) (== (`self.Alien Spawns Remaining`) 0))))

(fn `Register Alien Death`
  (params (Alien :type "/Game/Blueprints/AI/BP_Alien Object Reference (by ref)"))
  (`KismetArrayLibrary.Array_RemoveItem` (`self.Aliens`) Alien)
  (bind _returnvalue (`self.isWaveComplete`))
  (if _returnvalue
    (`self.End Wave`)))

(fn `Setup New Wave`
  (`/Engine/EditorBlueprintResources/StandardMacros.IncrementInt` (`self.Current Wave`)
    (:`  `
      (`KismetSystemLibrary.K2_SetTimer` null "Spawn Wave" 1.0 true))))

(fn `Spawn Alien`
  (bind _spawn_point (`self.Getrandomspawnpoint`))
  (`/Engine/EditorBlueprintResources/StandardMacros.IsValid` _spawn_point
    (:`Is Valid`
      (bind _returnvalue (`|SpawnActorFromClass` "/Game/Blueprints/AI/BP_Alien.BP_Alien_C" (`self.GetTransform` _spawn_point) "Undefined" "OverrideRootScale" null null))
      (`/Engine/EditorBlueprintResources/StandardMacros.IsValid` _returnvalue
        (:`Is Valid`
          (`KismetArrayLibrary.Array_Add` (`self.Aliens`) _returnvalue)
          (bind _result (`/Engine/EditorBlueprintResources/StandardMacros.DecrementInt` (`self.Alien Spawns Remaining`))
            (:`  `
              (if (== _result 0)
                (`KismetSystemLibrary.K2_ClearTimer` null "Spawn Wave")))))))))

(fn `Start New Wave`
  (`/Engine/EditorBlueprintResources/StandardMacros.IncrementInt` (`self.Current Wave`)
    (:`  `
      (`self.increasewavediff`)
      (`KismetSystemLibrary.K2_SetTimer` null "Spawn Wave" (`self.Spawn Freq`) true))))

(fn `UserConstructionScript`)